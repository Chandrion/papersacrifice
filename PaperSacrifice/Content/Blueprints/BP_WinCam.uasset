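; End-of-match camera actor that shows the win or lose screen and then reloads into the Arena level.
; Victory and lose events each add their widget, then share one path that points every player controller's view at this actor and sets the Victory flag, even on a loss.
; While that flag is set, Tick slowly raises the camera and opens Arena after a few seconds.
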(event `self.ReceiveTick`
  (params (DeltaSeconds :type "Float (single-precision)"))
  (bind _timeelapsed (`self.TimeElapsed`))
  (if (`self.victory`)
    (`SceneComponent.K2_AddRelativeLocation` (`self.Camera`) (`KismetMathLibrary.MakeVector` 0.0 0.0 (* DeltaSeconds 5.0)) false false)
    (set `self.TimeElapsed` (+ _timeelapsed DeltaSeconds))
    (if (> _timeelapsed 5.0)
      (`GameplayStatics.OpenLevel` "Arena"))))

(event `OnVictory_Event`
  (bind _returnvalue (`|CreateWidget` "/Game/UI/VictoryScreen.VictoryScreen_C"))
  (`UserWidget.AddToViewport` _returnvalue 0)
  (bind _outactors (`GameplayStatics.GetAllActorsOfClass` "/Game/Blueprints/BP_PlayerController.BP_PlayerController_C" :!label _label))
  (for (_ _array_index) _outactors
    (`PlayerController.SetViewTargetWithBlend` (`GameplayStatics.GetPlayerController` _array_index) self 0.0 "VTBlend_Linear" 0.0 false)
    (set `self.victory` true)))

(event `LoseEvent_Event`
  (bind _returnvalue (`|CreateWidget` "/Game/UI/LoseScreen.LoseScreen_C"))
  (`UserWidget.AddToViewport` _returnvalue 0)
  (goto _label))

(fn `UserConstructionScript`)