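; BP_Player2 is a robot player character that moves on fixed world axes, lunges forward on jump and knocks other BP_Player2 characters around.
; Enhanced Input drives movement, a jump locked until landing, and a shovel attack gated by a timed cooldown.
; MeleeHitbox overlaps maintain the set of targets that the attack launches away after a short delay.
; Body collisions bounce the other player in proportion to this character's speed, unless that player is already moving fast.
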(event `self.ReceiveBeginPlay`
  (`|ExecutionSequence`
    (:`then_0`
      (bind _outactors (`GameplayStatics.GetAllActorsOfClass` "/Game/Blueprints/BP_Camera.BP_Camera_C"))
      (set `self.RefCamera` (`|GetArrayItem` _outactors)))
    (:`then_1`
      (`KismetSystemLibrary.DelayUntilNextTick`))
    (:`then_2`
      (bind _asbp_player_controller (cast `/Game/Blueprints/BP_PlayerController` (`GameplayStatics.GetPlayerController` (`self.PlayerIndex`)))
        (:`then`
          (bind _returnvalue (pcsubsystem `EnhancedInputLocalPlayerSubsystem` _asbp_player_controller))
          (`/Engine/EditorBlueprintResources/StandardMacros.IsValid` _returnvalue
            (:`Is Valid`
              (`EnhancedInputSubsystemInterface.AddMappingContext` _returnvalue "/Game/Input/IMC_PlayerBot.IMC_PlayerBot" 0 (struct)))
            (:`Is Not Valid`
              (`KismetSystemLibrary.PrintString` "Input missing" :!label _label))))
        (:`CastFailed`
          (goto _label))))))

(event `EnhancedInput|/Game/Input/IA_Moving`
  (params (ActionValue :type "Vector2D Structure") (ElapsedSeconds :type "Float (double-precision)") (TriggeredSeconds :type "Float (double-precision)") (InputAction :type "InputAction Object Reference" :default "/Game/Input/IA_Moving.IA_Moving"))
  (:`Triggered`
    (`self.AddMovementInput` (`KismetMathLibrary.GetRightVector` (struct :`Pitch` 180.0 :`Roll` 180.0)) ActionValue_X)
    (`self.AddMovementInput` (`KismetMathLibrary.GetForwardVector` (struct :`Pitch` 180.0 :`Roll` 180.0)) ActionValue_Y)))

(event `EnhancedInput|/Game/Input/IA_Attack`
  (params (ActionValue :type Boolean) (ElapsedSeconds :type "Float (double-precision)") (TriggeredSeconds :type "Float (double-precision)") (InputAction :type "InputAction Object Reference" :default "/Game/Input/IA_Attack.IA_Attack"))
  (:`Started`
    (if (`self.CanAttack`)
      (set `self.CanAttack` false)
      (`SkeletalMeshComponent.PlayAnimation` (`self.Mesh`) "/Game/Models/Robot/robot_anim_001_Anim_Robot_shovel_attack.robot_anim_001_Anim_Robot_shovel_attack" false)
      (`KismetSystemLibrary.Delay` 0.2)
      (bind _result (`BlueprintSetLibrary.Set_ToArray` (`self.TargetsInRange`)))
      (for _array_element _result
        (bind (_returnvalue_x _returnvalue_y) (`KismetMathLibrary.BreakVector` (* (`KismetMathLibrary.GetDirectionUnitVector` (`self.K2_GetActorLocation`) (`self.K2_GetActorLocation` _array_element)) (`self.MeleePower`))))
        (`self.LaunchCharacter` _array_element (+ (`KismetMathLibrary.MakeVector` _returnvalue_x _returnvalue_y) (0.0 0.0 100.0)) false false))
      (`KismetSystemLibrary.Delay` 0.8)
      (set `self.CanAttack` true))))

(event `self.OnLanded`
  (params (Hit :type "HitResult Structure (by ref)"))
  (set `self.Jumping` false))

(event `EnhancedInput|/Game/Input/IA_Jumping`
  (params (ActionValue :type Boolean) (ElapsedSeconds :type "Float (double-precision)") (TriggeredSeconds :type "Float (double-precision)") (InputAction :type "InputAction Object Reference" :default "/Game/Input/IA_Jumping.IA_Jumping"))
  (:`Started`
    (if (not (`self.Jumping`))
      (`self.LaunchCharacter` (+ (* (`SceneComponent.GetForwardVector` (`self.CapsuleComponent`)) (`self.JumpPower`)) (0.0 0.0 100.0)))
      (set `self.Jumping` true))))

(event `self.ReceiveHit`
  (params (MyComp :type "PrimitiveComponent Object Reference") (Other :type "Actor Object Reference") (OtherComp :type "PrimitiveComponent Object Reference") (bSelfMoved :type Boolean) (HitLocation :type "Vector Structure") (HitNormal :type "Vector Structure") (NormalImpulse :type "Vector Structure") (Hit :type "HitResult Structure (by ref)"))
  (bind _asbp_player_2 (cast `/Game/Blueprints/BP_Player2` Other))
  (if (not (> (`KismetMathLibrary.VSize` (`CharacterMovementComponent.GetLastUpdateVelocity` (`Character.CharacterMovement` _asbp_player_2))) 800.0))
    (bind (_returnvalue_x _returnvalue_y) (`KismetMathLibrary.BreakVector` (* (`KismetMathLibrary.GetDirectionUnitVector` (`self.K2_GetActorLocation`) (`self.K2_GetActorLocation` _asbp_player_2)) (`KismetMathLibrary.FMax` (* (`KismetMathLibrary.VSize` (`CharacterMovementComponent.GetLastUpdateVelocity` (`self.CharacterMovement`))) (`self.BounceFactor`))))))
    (`self.LaunchCharacter` _asbp_player_2 (+ (`KismetMathLibrary.MakeVector` _returnvalue_x _returnvalue_y) (0.0 0.0 100.0)) false false)))

(event `self.MeleeHitbox.OnComponentBeginOverlap`
  (params (OverlappedComponent :type "PrimitiveComponent Object Reference") (OtherActor :type "Actor Object Reference") (OtherComp :type "PrimitiveComponent Object Reference") (OtherBodyIndex :type Integer) (bFromSweep :type Boolean) (SweepResult :type "HitResult Structure (by ref)"))
  (bind _asbp_player_2 (cast `/Game/Blueprints/BP_Player2` OtherActor))
  (`BlueprintSetLibrary.Set_Add` (`self.TargetsInRange`) _asbp_player_2))

(event `self.MeleeHitbox.OnComponentEndOverlap`
  (params (OverlappedComponent :type "PrimitiveComponent Object Reference") (OtherActor :type "Actor Object Reference") (OtherComp :type "PrimitiveComponent Object Reference") (OtherBodyIndex :type Integer))
  (bind _asbp_player_2 (cast `/Game/Blueprints/BP_Player2` OtherActor))
  (`BlueprintSetLibrary.Set_Remove` (`self.TargetsInRange`) _asbp_player_2))

(fn `UserConstructionScript`)