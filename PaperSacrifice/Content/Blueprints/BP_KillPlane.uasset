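; BP_KillPlane is an overlap actor that counts each BP_Player2 that enters it as a kill and responds with shredder feedback.
; Each kill activates Niagara effects on two pipes and plays a shredder sound.
; Below four kills, it has the level's BP_Bridge spawn more parts in that player's color, then switches the effects off after a short delay.
; On the fourth kill, it opens the configured level.
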(event `self.ReceiveBeginPlay`
  (bind _returnvalue (`GameplayStatics.GetActorOfClass` "/Game/Blueprints/BP_Bridge.BP_Bridge_C"))
  (set `self.Bridge` _returnvalue))

(event `self.ReceiveActorBeginOverlap`
  (params (OtherActor :type "Actor Object Reference"))
  (bind _niagaracomponent (`NiagaraActor.NiagaraComponent` (`self.PipeRight`)))
  (bind _niagaracomponent_2 (`NiagaraActor.NiagaraComponent` (`self.PipeLeft`)))
  (bind _asbp_player_2 (cast `/Game/Blueprints/BP_Player2` OtherActor))
  (`/Engine/EditorBlueprintResources/StandardMacros.IncrementInt` (`self.Kills`)
    (:`  `
      (`KismetSystemLibrary.PrintString` "Kill!")
      (`ActorComponent.Activate` _niagaracomponent_2 false)
      (`ActorComponent.Activate` _niagaracomponent false)
      (`GameplayStatics.PlaySound2D` "/Game/Audio/Shredder.Shredder" 1.0 1.0 0.0 null null)
      (if (>= (`self.Kills`) 4)
        (`GameplayStatics.OpenLevel` (`self.Level`))
        (else
          (`/Game/Blueprints/BP_Bridge.Spawn More Parts` (`self.Bridge`) (`/Game/Blueprints/BP_Player2.GetMyColor` _asbp_player_2))
          (`KismetSystemLibrary.Delay` 1.0)
          (`ActorComponent.Deactivate` _niagaracomponent_2)
          (`ActorComponent.Deactivate` _niagaracomponent))))))

(fn `UserConstructionScript`)