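; Robot Blueprint that shows or hides its AMSpearsV001 weapon component based on the classic weapon selection.
; Every Tick it reads WeaponClassicSelectedID, makes the component visible only when the ID is zero, and prints a true/false debug string.
; The toggleweapon event is an empty stub, so visibility relies entirely on per-frame polling.
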(event `self.ReceiveTick`
  (params (DeltaSeconds :type "Float (single-precision)"))
  (bind _am_spears_v001 (`self.AM_Spears_v001`))
  (if (== (`/Game/UI/BP_Selection.WeaponClassicSelected_ID` (`self.Target`)) 0)
    (`SceneComponent.SetVisibility` _am_spears_v001 true false)
    (`KismetSystemLibrary.PrintString` "true")
    (else
      (`SceneComponent.SetVisibility` _am_spears_v001 false false)
      (`KismetSystemLibrary.PrintString` "false"))))

(event `toggle weapon`
  (params (`selected weapon` :type Integer)))

(fn `UserConstructionScript`)