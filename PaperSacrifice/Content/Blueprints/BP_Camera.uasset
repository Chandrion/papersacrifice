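; BP_Camera is a shared camera actor that also sets up four local players at BeginPlay.
; It creates any missing player controllers, spawns a BP_Player2 at each of the first four BP_SpawnPoints, possesses it, assigns its index and shows the cursor.
; It then sets itself as the view target for the player controllers.
; A spawn-point shuffle exists but is disconnected, so spawns follow the found actor order.
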(event `self.ReceiveBeginPlay`
  (bind _returnvalue (`GameplayStatics.GetPlayerController` (`self.SpawnIndex`)))
  (bind _outactors (`GameplayStatics.GetAllActorsOfClass` "/Game/Blueprints/BP_SpawnPoints.BP_SpawnPoints_C"))
  (bind _output_get (set `self.SpawnPoints` _outactors))
  (for _index (range 4)
    (bind _output_get_2 (set `self.SpawnIndex` _index))
    (`/Engine/EditorBlueprintResources/StandardMacros.IsValid` (`GameplayStatics.GetPlayerController` _output_get_2)
      (:`Is Valid`
        _)
      (:`Is Not Valid`
        (`GameplayStatics.CreatePlayer` (`self.SpawnIndex`))))
    (bind _returnvalue_2 (`|SpawnActorFromClass` "/Game/Blueprints/BP_Player2.BP_Player2_C" (`self.GetTransform` (`|GetArrayItem` (`self.SpawnPoints`) (`self.SpawnIndex`))) "AlwaysSpawn" "MultiplyWithRoot" null null))
    (`Controller.Possess` _returnvalue _returnvalue_2)
    (set `/Game/Blueprints/BP_Player2.PlayerIndex` (`self.SpawnIndex`) _returnvalue_2)
    (set `PlayerController.bShowMouseCursor` true _returnvalue))
  (bind _outactors_2 (`GameplayStatics.GetAllActorsOfClass` "/Game/Blueprints/BP_PlayerController.BP_PlayerController_C"))
  (for (_ _array_index) _outactors_2
    (`PlayerController.SetViewTargetWithBlend` (`GameplayStatics.GetPlayerController` _array_index) self 0.0 "VTBlend_Linear" 0.0 false)))

(fn `UserConstructionScript`)